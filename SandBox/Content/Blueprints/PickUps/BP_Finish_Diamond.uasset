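; BP_Finish_Diamond is a finish pickup that awards score and brings up the end menu when collected.
; PickupDiamond passes its Value to BP_MyGamemode's UpdateScore and destroys its mesh component, leaving the actor alive through a short delay.
; It then calls SetEndMenuText with true on BP_EndMenu and has the game mode swap the HUD for that menu, showing the cursor and disabling input.
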(event EventPickupDiamond
  (params (Player :type My%20Player%20Object%20Reference))
  ;[0.15 0.15 0.15 0.5] Update Score and destroys this object
  (bind _asbp_my_gamemode (Utilities|Casting|CastToBP_MyGamemode (Game|GetGameMode)))
  (Class|MyGameModeBase|UpdateScore _asbp_my_gamemode (Variables|Default|GetValue))
  (Components|DestroyComponent (Variables|Character|GetMesh))
  (Utilities|FlowControl|Delay 0.7)
  (bind _asbp_my_gamemode_2 (Utilities|Casting|CastToBP_MyGamemode (Game|GetGameMode)))
  (bind _asbp_end_menu (Utilities|Casting|CastToBP_EndMenu (Variables|/Script/SandBox.MyGameModeBase|GetEndMenuRef _asbp_my_gamemode_2)))
  (Default|SetEndMenuText _asbp_end_menu true)
  (Class|MyGameModeBase|AddRemoveUI _asbp_my_gamemode_2 true true (Variables|/Script/SandBox.MyGameModeBase|GetGameHUDRef _asbp_my_gamemode_2) (Variables|/Script/SandBox.MyGameModeBase|GetEndMenuRef _asbp_my_gamemode_2)))

(fn ConstructionScript)